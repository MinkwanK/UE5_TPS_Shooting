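; Enemy AI Blueprint that detects the player through AI Perception and relays target state to its AIC_EnemyAI controller.
; Sensing a Player-tagged actor cancels the loss timer, then sets the target and line-of-sight key.
; Any other perception update clears line of sight and starts a five-second timer, after which the target is cleared.
; RandomWander is empty, with leftover timer and random-move nodes left unconnected.
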(event `Random Wander`
  ;[1 1 1] 무작위 이동
)

(event `self.ReceiveBeginPlay`
  ;[1 1 1] 무작위 이동
)

(event `self.AIPerception.OnTargetPerceptionUpdated`
  (params (Actor :type "Actor Object Reference") (Stimulus :type "AIStimulus Structure"))
  (bind _output_get (set `self.PerceivedActor` Actor))
  (if (and (`self.ActorHasTag` _output_get "Player") (`.bSuccessfullySensed` (break `AIStimulus` Stimulus)))
    (`KismetSystemLibrary.K2_ClearAndInvalidateTimerHandle` (`self.TargetLost Timer`))
    (`/Game/Enemy/AI/AIC_EnemyAI.Update Target Actor` (cast `/Game/Enemy/AI/AIC_EnemyAI` (`self.GetController`) :!pure true) (`self.PerceivedActor`))
    (`/Game/Enemy/AI/AIC_EnemyAI.Update Has Line Of Sight to Key` (cast `/Game/Enemy/AI/AIC_EnemyAI` (`self.GetController`) :!pure true) true)
    (else
      (bind _returnvalue (`KismetSystemLibrary.K2_SetTimerDelegate` (delegate `TargetLost`) 5.0))
      (set `self.TargetLost Timer` _returnvalue)
      (`/Game/Enemy/AI/AIC_EnemyAI.Update Has Line Of Sight to Key` (cast `/Game/Enemy/AI/AIC_EnemyAI` (`self.GetController`) :!pure true) false))))

(event `TargetLost`
  (set `self.PerceivedActor` null)
  (`/Game/Enemy/AI/AIC_EnemyAI.Update Target Actor` (cast `/Game/Enemy/AI/AIC_EnemyAI` (`self.GetController`) :!pure true) null) ; 타겟 액터 무효화이므로 타겟 액터에 아무것도 넣지 않는다
)

(fn `UserConstructionScript`)